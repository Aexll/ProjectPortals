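; BP_Enemy is an AI-controlled enemy pawn with an AIPerception component.
; On BeginPlay it casts its controller to AIController and initializes the BB_Enemy blackboard, without starting a behavior tree here.
; The perception event handlers are empty.
; A disconnected, never-executed chain sketches moving to a stimulus location, requesting a prediction of the target's position, then refreshing the perception listener after a delay.
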(event `self.ReceiveBeginPlay`
  (bind _asaicontroller (cast `AIController` (`self.GetController`)))
  (`AIController.UseBlackboard` _asaicontroller "/Game/Enemy/BB_Enemy.BB_Enemy"))

(event `self.AIPerception.OnPerceptionUpdated`
  (params (UpdatedActors :type "Array of Actor Object Reference (by ref)")))

(event `self.AIPerception.OnTargetPerceptionInfoUpdated`
  (params (UpdateInfo :type "ActorPerceptionUpdateInfo Structure (by ref)")))

(event `self.AIPerception.OnTargetPerceptionUpdated`
  (params (Actor :type "Actor Object Reference") (Stimulus :type "AIStimulus Structure")))

(fn `UserConstructionScript`)